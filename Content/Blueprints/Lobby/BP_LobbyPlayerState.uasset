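; Lobby player state that holds a player's name and selected class index.
; On BeginPlay it reads PlayerId from BP_GameInstance, passes it to ServerSetPlayerName as the player name and prints it, with no local-ownership check.
; ServerCycleClassIndex steps ClassIndex through the ClassNames array, wrapping to zero after the last entry.
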(event `ServerCycleClassIndex`
  (if (< (`self.ClassIndex`) (- (`KismetArrayLibrary.Array_Length` (`self.ClassNames`)) 1))
    (`/Engine/EditorBlueprintResources/StandardMacros.IncrementInt` (`self.ClassIndex`))
    (else
      (set `self.ClassIndex` 0))))

(event `ServerSetPlayerName`
  (params (PlayerName :type String))
  (set `self.PlayerName` PlayerName))

(event `self.ReceiveBeginPlay`
  (`self.LocalSetPlayerName`))

(event `LocalSetPlayerName`
  (bind _asbp_game_instance (cast `/Game/Blueprints/BP_GameInstance` (`GameplayStatics.GetGameInstance`)))
  (bind _playerid (`/Game/Blueprints/BP_GameInstance.PlayerId` _asbp_game_instance))
  (`self.ServerSetPlayerName` _playerid)
  (`KismetSystemLibrary.PrintString` (`KismetStringLibrary.Concat_StrStr` "Setting player name to: " _playerid)))

(fn `UserConstructionScript`)