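; Lobby game mode that assigns joining players to one of two teams and launches the match.
; On post-login it notifies BP_LobbyGameState, then gives the new player's BP_LobbyPlayerState the TeamId of the smaller team, counted from the PlayerArray, with ties going to team 1.
; Logouts are also forwarded to the game state.
; A start request triggers a servertravel console command to MAP_Match.
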(event `self.K2_PostLogin`
  (params (NewPlayer :type "PlayerController Object Reference"))
  (bind _asbp_lobby_game_state (cast `/Game/Blueprints/Lobby/BP_LobbyGameState` (`GameplayStatics.GetGameState`)))
  (`/Game/Blueprints/Lobby/BP_LobbyGameState.OnPostLogin` _asbp_lobby_game_state)
  (bind _teamid (`self.WhichTeamShouldPlayerBeAddedTo`))
  (bind _asbp_lobby_player_state (cast `/Game/Blueprints/Lobby/BP_LobbyPlayerState` (`Controller.PlayerState` NewPlayer)))
  (set `/Game/Blueprints/Lobby/BP_LobbyPlayerState.TeamId` _teamid _asbp_lobby_player_state))

(event `self.K2_OnLogout`
  (params (ExitingController :type "Controller Object Reference"))
  (bind _asbp_lobby_game_state (cast `/Game/Blueprints/Lobby/BP_LobbyGameState` (`GameplayStatics.GetGameState`)))
  (`/Game/Blueprints/Lobby/BP_LobbyGameState.OnPostLogout` _asbp_lobby_game_state))

(event `RequestStartGame`
  (`KismetSystemLibrary.PrintString` "Request Start Game")
  (`KismetSystemLibrary.ExecuteConsoleCommand` "servertravel MAP_Match" null))

(fn `UserConstructionScript`)

(fn `WhichTeamShouldPlayerBeAddedTo`
  (returns (TeamId :type Integer))
  (locals (TeamACount :type Integer) (TeamBCount :type Integer))
  (for _array_element (`GameStateBase.PlayerArray` (`GameplayStatics.GetGameState`))
    (bind _asbp_lobby_player_state (cast `/Game/Blueprints/Lobby/BP_LobbyPlayerState` _array_element))
    (bind _teamid (`/Game/Blueprints/Lobby/BP_LobbyPlayerState.TeamId` _asbp_lobby_player_state))
    (if (== _teamid 1)
      (`/Engine/EditorBlueprintResources/StandardMacros.IncrementInt` (`local.TeamACount`))
      (elif (== _teamid 2)
        (`/Engine/EditorBlueprintResources/StandardMacros.IncrementInt` (`local.TeamBCount`)))))
  (if (< (`local.TeamBCount`) (`local.TeamACount`))
    (return 2)
    (else
      (return 1))))